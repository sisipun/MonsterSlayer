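; Base melee attack Gameplay Ability that plays an attack montage and applies a hit to the struck target.
; After commit, it waits for a single Ability.Attack.Hit gameplay event, then applies GE_Hit to the payload's target data.
; The hit also reports a damage event to AI perception at the instigator's location.
; The ability ends when the montage completes, blends out or is interrupted, ending the stored wait task.
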(event Ability|EventActivateAbility
  (bind _returnvalue (Ability|CommitAbility))
  (if _returnvalue
    (Animation|Montage|PlayMontage (.skeletalmeshcomponent (Ability|GetActorInfo)) (Variables|Default|GetMontage)
      (:then
        (bind (_asynctaskproxy _payload) (Ability|Tasks|WaitGameplayEvent "(TagName=\"Ability.Attack.Hit\")" 0 true)
          (:then
            (Variables|Default|SetTask _asynctaskproxy))
          (:EventReceived
            (GameplayEffects|ApplyGameplayEffectToTarget (.TargetData (Utilities|Struct|BreakGameplayEventData _payload)) "/Game/Ability/Shared/GE_Hit.GE_Hit_C" 1 1)
            (Class|AISenseDamage|ReportDamageEvent (.Target (Utilities|Struct|BreakGameplayEventData _payload)) (.Instigator (Utilities|Struct|BreakGameplayEventData _payload)) 1.0 (Transformation|GetActorLocation (.Instigator (Utilities|Struct|BreakGameplayEventData _payload)))))))
      (:OnCompleted
        (Ability|EndAbility :!label _label))
      (:OnBlendOut
        (goto _label))
      (:OnInterrupted
        (goto _label)))
    (else
      (Ability|EndAbility))))

(event Ability|EventOnEndAbility
  (params (bWasCancelled :type Boolean))
  (bind _task (Variables|Default|GetTask))
  (Utilities|IsValid _task
    (:Is%20Valid
      (GameplayTasks|EndTask _task))))