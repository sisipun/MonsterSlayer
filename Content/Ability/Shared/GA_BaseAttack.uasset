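; Shared base melee-style attack Gameplay Ability that plays a combo montage on a BaseCharacter and applies hit effects.
; After commit, it waits for hit-tag gameplay events, applying GE_Hit to the target data and reporting a damage event for AI perception.
; A DoOnce limits hits to one per swing; montage notifies reset it when a combo is queued, otherwise they blend the montage out.
; The ability ends with the montage and cleans up the event task.
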(event Ability|EventActivateAbility
  (bind _returnvalue (Ability|GetActorInfo))
  (bind _asbase_character (Utilities|Casting|CastToBaseCharacter (.avataractor _returnvalue))
    (:then
      (Variables|Default|SetCharacter _asbase_character)
      (bind _returnvalue_2 (Ability|CommitAbility))
      (if _returnvalue_2
        (Animation|Montage|PlayMontage (.skeletalmeshcomponent _returnvalue) (Variables|Default|GetMontage)
          (:then
            (bind (_asynctaskproxy _payload) (Ability|Tasks|WaitGameplayEvent (Variables|Default|GetHitTag) 0)
              (:then
                (Variables|Default|SetTask _asynctaskproxy))
              (:EventReceived
                (Utilities|FlowControl|DoOnce false :!label _label
                  (:Completed
                    (GameplayEffects|ApplyGameplayEffectToTarget (.TargetData (Utilities|Struct|BreakGameplayEventData _payload)) "/Game/Ability/Shared/GE_Hit.GE_Hit_C" 1 1)
                    (Class|AISenseDamage|ReportDamageEvent (.Target (Utilities|Struct|BreakGameplayEventData _payload)) (.Instigator (Utilities|Struct|BreakGameplayEventData _payload)) 1.0 (Transformation|GetActorLocation (.Instigator (Utilities|Struct|BreakGameplayEventData _payload)))))))))
          (:OnCompleted
            (Ability|EndAbility :!label _label_2))
          (:OnBlendOut
            (goto _label_2))
          (:OnInterrupted
            (goto _label_2))
          (:OnNotifyBegin
            (if (Variables|/Script/MonsterSlayer.BaseCharacter|GetbAttackComboActivated (Variables|Default|GetCharacter))
              (Variables|/Script/MonsterSlayer.BaseCharacter|SetbAttackComboActivated (Variables|Default|GetCharacter) false)
              (goto _label Reset)
              (else
                (Animation|Montage|MontageStop (Components|SkeletalMesh|GetAnimInstance (Variables|/Script/Engine.Character|GetMesh (Variables|Default|GetCharacter))) 1.0 (Variables|Default|GetMontage))))))
        (else
          (Ability|EndAbility))))
    (:CastFailed
      (Ability|EndAbility))))

(event Ability|EventOnEndAbility
  (params (bWasCancelled :type Boolean))
  (bind _task (Variables|Default|GetTask))
  (Utilities|IsValid _task
    (:Is%20Valid
      (GameplayTasks|EndTask _task))))