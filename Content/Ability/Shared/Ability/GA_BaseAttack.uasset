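; Base melee attack ability that plays a combo montage and damages the enemy character reported by a hit gameplay event.
; Each montage notify either consumes the combo flag and re-arms the once-only hit gate, or blends the montage out.
; Hits skip dead or same-team targets, apply GE_Hit and report an AI damage event.
; A killing hit triggers the attacker's Reaction.Kill ability; montage end closes the ability.
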(event Ability|EventActivateAbility
  (bind _returnvalue (Ability|GetActorInfo))
  (bind _asbase_character (Utilities|Casting|CastToBaseCharacter (.avataractor _returnvalue))
    (:then
      (Variables|Default|SetCharacter _asbase_character)
      (bind _returnvalue_2 (Ability|CommitAbility))
      (if _returnvalue_2
        (Animation|Montage|PlayMontage (.skeletalmeshcomponent _returnvalue) (Variables|Default|GetMontage)
          (:then
            (bind (_asynctaskproxy _payload) (Ability|Tasks|WaitGameplayEvent (Variables|Default|GetHitTag) 0)
              (:then
                (Variables|Default|SetTask _asynctaskproxy))
              (:EventReceived
                (Utilities|FlowControl|DoOnce false :!label _label
                  (:Completed
                    (bind _isdead (CallFunction|ApplyDamage _payload))
                    (if _isdead
                      (Class|BaseCharacter|ActivateAbilitieswithTags (Variables|Default|GetCharacter) "(GameplayTags=((TagName=\"Reaction.Kill\")))")))))))
          (:OnCompleted
            (Ability|EndAbility :!label _label_2))
          (:OnBlendOut
            (goto _label_2))
          (:OnInterrupted
            (goto _label_2))
          (:OnNotifyBegin
            (if (Variables|/Script/MonsterSlayer.BaseCharacter|GetbAttackComboActivated (Variables|Default|GetCharacter))
              (Variables|/Script/MonsterSlayer.BaseCharacter|SetbAttackComboActivated (Variables|Default|GetCharacter) false)
              (goto _label Reset)
              (else
                (Animation|Montage|MontageStop (Components|SkeletalMesh|GetAnimInstance (Variables|/Script/Engine.Character|GetMesh (Variables|Default|GetCharacter))) 1.0 (Variables|Default|GetMontage))))))
        (else
          (Ability|EndAbility))))
    (:CastFailed
      (Ability|EndAbility))))

(event Ability|EventOnEndAbility
  (params (bWasCancelled :type Boolean))
  (bind _task (Variables|Default|GetTask))
  (Utilities|IsValid _task
    (:Is%20Valid
      (GameplayTasks|EndTask _task))))

(fn ApplyDamage
  (params (GameplayEventData :type Gameplay%20Event%20Data%20Structure%20%28by%20ref%29))
  (bind (_eventtag _instigator _target _optionalobject _optionalobject2 _contexthandle _instigatortags _targettags _eventmagnitude _targetdata) (Utilities|Struct|BreakGameplayEventData GameplayEventData))
  (bind _asbase_character (Utilities|Casting|CastToBaseCharacter _instigator)
    (:then
      (LocalVariables|SetSource _asbase_character)
      (bind _asbase_character_2 (Utilities|Casting|CastToBaseCharacter _target)
        (:then
          (bind _output_get (LocalVariables|SetTarget _asbase_character_2))
          (if (Class|BaseCharacter|IsDead _output_get)
            (return false)
            (else
              (bind _same (CallFunction|HasSameTeam (LocalVariables|GetSource) (LocalVariables|GetTarget)))
              (if _same
                (return false)
                (else
                  (GameplayEffects|ApplyGameplayEffectToTarget _targetdata "/Game/Ability/Shared/Effect/GE_Hit.GE_Hit_C" (Class|BaseCharacter|GetLevel (LocalVariables|GetSource)) 1)
                  (Class|AISenseDamage|ReportDamageEvent (LocalVariables|GetTarget) (LocalVariables|GetSource) 1.0 (Transformation|GetActorLocation (LocalVariables|GetSource)))
                  (return (Class|BaseCharacter|IsDead (LocalVariables|GetTarget))))))))
        (:CastFailed
          (return false))))
    (:CastFailed
      (return false))))

(fn HasSameTeam
  (params (First :type Actor%20Object%20Reference) (Second :type Actor%20Object%20Reference))
  (bind _asbase_character (Utilities|Casting|CastToBaseCharacter First)
    (:then
      (bind _asbase_character_2 (Utilities|Casting|CastToBaseCharacter Second)
        (:then
          (return (== (Utilities|Struct|BreakGenericTeamId (Class|BaseCharacter|GetGenericTeamId _asbase_character)) (Utilities|Struct|BreakGenericTeamId (Class|BaseCharacter|GetGenericTeamId _asbase_character_2)))))
        (:CastFailed
          (return false))))
    (:CastFailed
      (return false))))