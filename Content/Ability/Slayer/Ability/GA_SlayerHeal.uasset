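; Gameplay Ability that lets the Slayer heal itself, with the heal scaled by experience level.
; After casting the avatar to Slayer and committing the ability, it starts the heal montage and immediately applies GE_Heal to the owner, using experience level as the stack count.
; The ability ends when the montage completes, blends out or is interrupted, or right away if the cast or commit fails.
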(event Ability|EventActivateAbility
  (bind _returnvalue (Ability|GetActorInfo))
  (bind _asslayer (Utilities|Casting|CastToSlayer (.avataractor _returnvalue))
    (:then
      (Variables|Default|SetSlayer _asslayer)
      (bind _returnvalue_2 (Ability|CommitAbility))
      (if _returnvalue_2
        (Animation|Montage|PlayMontage (.skeletalmeshcomponent _returnvalue) "/Game/Character/Slayer/Animations/AM_Slayer_Heal.AM_Slayer_Heal"
          (:then
            (Ability|ApplyGameplayEffectToOwner "/Game/Ability/Shared/Effect/GE_Heal.GE_Heal_C" 1 (Class|BaseCharacter|GetExperienceLevel (Variables|Default|GetSlayer))))
          (:OnCompleted
            (Ability|EndAbility :!label _label))
          (:OnBlendOut
            (goto _label))
          (:OnInterrupted
            (goto _label)))
        (else
          (Ability|EndAbility))))
    (:CastFailed
      (Ability|EndAbility))))

(event Ability|EventOnEndAbility
  (params (bWasCancelled :type Boolean)))