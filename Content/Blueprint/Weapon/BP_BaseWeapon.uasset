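; BP_BaseWeapon is a base weapon that damages characters touched by its Collider.
; On begin overlap it filters for a BaseCharacter other than its Instigator, then applies Power as damage.
; It also reports the hit to AI damage perception, using the Instigator's location as the event location.
; A single DoOnce gates hits and resets when any overlap ends, rather than tracking each target.
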(event OnComponentBeginOverlap(Collider)
  (params (OverlappedComponent :type Primitive%20Component%20Object%20Reference) (OtherActor :type Actor%20Object%20Reference) (OtherComp :type Primitive%20Component%20Object%20Reference) (OtherBodyIndex :type Integer) (bFromSweep :type Boolean) (SweepResult :type Hit%20Result%20Structure%20%28by%20ref%29))
  (bind _asbase_character (Utilities|Casting|CastToBaseCharacter OtherActor))
  (if (!= _asbase_character (Game|GetInstigator))
    (Variables|Default|SetTarget _asbase_character)
    (Utilities|FlowControl|DoOnce false
      (:Completed
        (Game|Damage|ApplyDamage (Variables|Default|GetTarget) (Variables|Default|GetPower) 0 (Game|GetInstigator))
        (Class|AISenseDamage|ReportDamageEvent (Variables|Default|GetTarget) (Game|GetInstigator) (Variables|Default|GetPower) (Transformation|GetActorLocation (Game|GetInstigator)))))))

(event OnComponentEndOverlap(Collider)
  (params (OverlappedComponent :type Primitive%20Component%20Object%20Reference) (OtherActor :type Actor%20Object%20Reference) (OtherComp :type Primitive%20Component%20Object%20Reference) (OtherBodyIndex :type Integer))
  (Utilities|FlowControl|DoOnce false) ; enters at Reset
)

(fn ConstructionScript)