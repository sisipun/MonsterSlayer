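; Base weapon Blueprint that damages Monster actors during an attack.
; BeginWeaponAttack and EndWeaponAttack switch the Collider between query-only and no collision, which starts disabled at BeginPlay.
; Overlapping a Monster calls Hit with the weapon's Power through a DoOnce gate.
; That single gate is shared across all monsters and resets when any Monster ends overlap, limiting repeat hits.
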(event OnComponentBeginOverlap(Collider)
  (params (OverlappedComponent :type Primitive%20Component%20Object%20Reference) (OtherActor :type Actor%20Object%20Reference) (OtherComp :type Primitive%20Component%20Object%20Reference) (OtherBodyIndex :type Integer) (bFromSweep :type Boolean) (SweepResult :type Hit%20Result%20Structure%20%28by%20ref%29))
  (bind _asmonster (Utilities|Casting|CastToMonster OtherActor))
  (Utilities|FlowControl|DoOnce false
    (:Completed
      (Class|Monster|Hit _asmonster (Variables|Default|GetPower)))))

(event OnComponentEndOverlap(Collider)
  (params (OverlappedComponent :type Primitive%20Component%20Object%20Reference) (OtherActor :type Actor%20Object%20Reference) (OtherComp :type Primitive%20Component%20Object%20Reference) (OtherBodyIndex :type Integer))
  (Utilities|Casting|CastToMonster OtherActor)
  (Utilities|FlowControl|DoOnce false) ; enters at Reset
)

(event Custom|Event%20BeginWeaponAttack
  (Collision|SetCollisionEnabled (Variables|Default|GetCollider) "QueryOnly"))

(event Custom|Event%20EndWeaponAttack
  (Collision|SetCollisionEnabled (Variables|Default|GetCollider) "NoCollision"))

(event EventBeginPlay
  (Collision|SetCollisionEnabled (Variables|Default|GetCollider) "NoCollision")
  (Development|PrintString "1"))

(fn ConstructionScript)