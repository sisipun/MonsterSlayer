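; Slayer Blueprint that handles weapon cycling and timed attacks from player input.
; E and Q step an index forward or back through the Weapons array with wraparound, then pass it to ChangeWeapon, which is not defined here.
; Attack casts CurrentWeapon to BaseWeapon_BP and fires its begin and end attack events around a fixed delay.
; An IsAttacking flag blocks switching and repeat attacks during that window.
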(event EventBeginPlay
  (Variables|Weapon|SetCurrent%20Weapon%20Index 0))

(event Input|ActionEvents|InputActionAttack
  (params (Key :type Key%20Structure :default "None"))
  (:Pressed
    (if (not (Variables|State|GetIs%20Attacking))
      (Variables|State|SetIs%20Attacking true)
      (bind _weapon (Weapon|GetCurrentBaseWeapon))
      (Default|EventBeginWeaponAttack _weapon)
      (Utilities|FlowControl|Delay 1.0)
      (bind _weapon_2 (Weapon|GetCurrentBaseWeapon))
      (Default|EventEndWeaponAttack _weapon_2)
      (Variables|State|SetIs%20Attacking false))))

(event Input|KeyboardEvents|E
  (params (Key :type Key%20Structure :default "None"))
  (:Pressed
    (if (not (Variables|State|GetIs%20Attacking))
      (Weapon|SetNextCurrentWeaponIndex)
      (Class|Slayer|ChangeWeapon (Variables|Weapon|GetCurrent%20Weapon%20Index)))))

(event Input|KeyboardEvents|Q
  (params (Key :type Key%20Structure :default "None"))
  (:Pressed
    (if (not (Variables|State|GetIs%20Attacking))
      (Weapon|SetPreviousCurrentWeaponIndex)
      (Class|Slayer|ChangeWeapon (Variables|Weapon|GetCurrent%20Weapon%20Index))
      (bind _asbase_weapon_bp (Utilities|Casting|CastToBaseWeapon_BP (Variables|Default|GetCurrentWeapon)))
      (Variables|Weapon|SetCurrent%20Base%20Weapon _asbase_weapon_bp))))

(fn ConstructionScript)

(fn SetNextCurrentWeaponIndex
  (bind _result (Math|Integer|IncrementInt (Variables|Weapon|GetCurrent%20Weapon%20Index))
    (:%20%20
      (if (>= _result (Utilities|Array|Length (Variables|Default|GetWeapons)))
        (Variables|Weapon|SetCurrent%20Weapon%20Index 0)
        (else
          (Variables|Weapon|SetCurrent%20Weapon%20Index _result))))))

(fn SetPreviousCurrentWeaponIndex
  (bind _result (Math|Integer|DecrementInt (Variables|Weapon|GetCurrent%20Weapon%20Index))
    (:%20%20
      (if (< _result 0)
        (Variables|Weapon|SetCurrent%20Weapon%20Index (- (Utilities|Array|Length (Variables|Default|GetWeapons)) 1))
        (else
          (Variables|Weapon|SetCurrent%20Weapon%20Index _result))))))

(fn GetCurrentWeaponType
  (return (Utilities|Array|Get(acopy) (Variables|Default|GetWeapons) (Variables|Weapon|GetCurrent%20Weapon%20Index))))

(fn GetCurrentBaseWeapon
  (bind _asbase_weapon_bp (Utilities|Casting|CastToBaseWeapon_BP (Variables|Default|GetCurrentWeapon)))
  (bind _output_get (Variables|Weapon|SetCurrent%20Base%20Weapon _asbase_weapon_bp))
  (return _output_get))