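; Slayer Blueprint that handles player input for cycling weapons and attacking.
; E and Q step CurrentWeaponIndex forward or back through the Weapons array with wraparound, then call ChangeWeapon, but only while not attacking.
; The Attack input action calls Attack; that function, ChangeWeapon and IsAttacking are not defined in these graphs.
; A helper returns the weapon type at the current index.
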(event EventBeginPlay
  (Variables|Weapon|SetCurrent%20Weapon%20Index 0))

(event Input|ActionEvents|InputActionAttack
  (params (Key :type Key%20Structure :default "None"))
  (:Pressed
    (Class|BaseCharacter|Attack)))

(event Input|KeyboardEvents|E
  (params (Key :type Key%20Structure :default "None"))
  (:Pressed
    (if (not (Class|BaseCharacter|IsAttacking))
      (Weapon|SetNextCurrentWeaponIndex)
      (Class|BaseCharacter|ChangeWeapon (Variables|Weapon|GetCurrent%20Weapon%20Index)))))

(event Input|KeyboardEvents|Q
  (params (Key :type Key%20Structure :default "None"))
  (:Pressed
    (if (not (Class|BaseCharacter|IsAttacking))
      (Weapon|SetPreviousCurrentWeaponIndex)
      (Class|BaseCharacter|ChangeWeapon (Variables|Weapon|GetCurrent%20Weapon%20Index)))))

(fn ConstructionScript)

(fn SetNextCurrentWeaponIndex
  (bind _result (Math|Integer|IncrementInt (Variables|Weapon|GetCurrent%20Weapon%20Index))
    (:%20%20
      (if (>= _result (Utilities|Array|Length (Variables|Default|GetWeapons)))
        (Variables|Weapon|SetCurrent%20Weapon%20Index 0)
        (else
          (Variables|Weapon|SetCurrent%20Weapon%20Index _result))))))

(fn SetPreviousCurrentWeaponIndex
  (bind _result (Math|Integer|DecrementInt (Variables|Weapon|GetCurrent%20Weapon%20Index))
    (:%20%20
      (if (< _result 0)
        (Variables|Weapon|SetCurrent%20Weapon%20Index (- (Utilities|Array|Length (Variables|Default|GetWeapons)) 1))
        (else
          (Variables|Weapon|SetCurrent%20Weapon%20Index _result))))))

(fn GetCurrentWeaponType
  (return (Utilities|Array|Get(acopy) (Variables|Default|GetWeapons) (Variables|Weapon|GetCurrent%20Weapon%20Index))))