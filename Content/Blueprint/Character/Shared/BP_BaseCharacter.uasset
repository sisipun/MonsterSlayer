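; BP_BaseCharacter is a shared base character Blueprint that uses the Gameplay Ability System for melee punch attacks.
; BeginPunch runs a sphere overlap for pawns at the right-hand socket, ignoring itself.
; It sends the first hit to itself as a punch-hit gameplay event with target data, for abilities to handle.
; IsAttacking reports whether any active ability carries the Ability.Attack tag.
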(event EventBeginPunch
  (bind _self self)
  (bind _outactors (Collision|SphereOverlapActors (Transformation|GetSocketLocation (Variables|Character|GetMesh) "RightHand") 3e+01 (Utilities|Array|MakeArray "ObjectTypeQuery3") 0 (Utilities|Array|MakeArray self)))
  (if (Utilities|Array|IsValidIndex _outactors)
    (Ability|SendGameplayEventtoActor _self "(TagName=\"Ability.Attack.Punch.Hit\")" (Utilities|Struct|MakeGameplayEventData "" _self (Utilities|Array|Get(acopy) _outactors) 0 0 "()" "(GameplayTags=)" "(GameplayTags=)" 0.0 (Ability|TargetData|AbilityTargetDatafromActor (Utilities|Array|Get(acopy) _outactors))))))

(fn ConstructionScript)

(fn IsAttacking
  (return (> (Utilities|Array|Length (Class|CharacterAbilitySystemComponent|GetActiveAbilitieswithTags (Variables|Default|GetAbilitySystemComponent) (Utilities|Array|MakeArray "(GameplayTags=((TagName=\"Ability.Attack\")))"))) 0)))