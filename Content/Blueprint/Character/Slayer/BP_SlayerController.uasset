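; BP_SlayerController is the player controller for the Slayer character, creating its stats HUD and caching the possessed Slayer.
; Input actions activate Gameplay Ability System abilities on the Slayer by tag for rolling, healing, and changing or removing the current weapon.
; Attack picks a melee or punch ability based on whether a weapon is equipped, or flags a combo continuation if an attack is already running.
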(event EventBeginPlay
  (bind _returnvalue (Game|ConstructObjectfromClass "/Game/Blueprint/Character/Slayer/WB_SlayerStats.WB_SlayerStats_C" self))
  (bind _output_get (Variables|UI|SetSlayerUI _returnvalue))
  (Variables|/Game/Blueprint/Character/Slayer/WB_SlayerStats.WB_SlayerStats_C|SetSlayerController _output_get self)
  (UserInterface|Viewport|AddtoViewport _output_get 0))

(event EventPossess
  (params (PossessedPawn :type Pawn%20Object%20Reference))
  (bind _asslayer (Utilities|Casting|CastToSlayer PossessedPawn))
  (Variables|Default|SetSlayer _asslayer))

(event Input|ActionEvents|InputActionRoll
  (params (Key :type Key%20Structure :default "None"))
  (:Pressed
    (Class|BaseCharacter|ActivateAbilitieswithTags (Variables|Default|GetSlayer) "(GameplayTags=((TagName=\"Ability.Roll\")))")))

(event Input|ActionEvents|InputActionAttack
  (params (Key :type Key%20Structure :default "None"))
  (bind _slayer (Variables|Default|GetSlayer))
  (:Pressed
    (if (Class|BaseCharacter|IsAttacking (Variables|Default|GetSlayer))
      (Variables|/Script/MonsterSlayer.BaseCharacter|SetbAttackComboActivated _slayer true)
      (else
        (Utilities|IsValid (Variables|/Script/MonsterSlayer.BaseCharacter|GetCurrentWeapon _slayer)
          (:Is%20Valid
            (Class|BaseCharacter|ActivateAbilitieswithTags (Variables|Default|GetSlayer) "(GameplayTags=((TagName=\"Ability.Attack.Melee\")))"))
          (:Is%20Not%20Valid
            (Class|BaseCharacter|ActivateAbilitieswithTags (Variables|Default|GetSlayer) "(GameplayTags=((TagName=\"Ability.Attack.Punch\")))")))))))

(event Input|ActionEvents|InputActionAbility
  (params (Key :type Key%20Structure :default "None"))
  (:Pressed
    (Class|BaseCharacter|ActivateAbilitieswithTags (Variables|Default|GetSlayer) "(GameplayTags=((TagName=\"Ability.Heal\")))")))

(event Input|ActionEvents|InputActionCurrentWeaponChange
  (params (Key :type Key%20Structure :default "None"))
  (:Pressed
    (Class|BaseCharacter|ActivateAbilitieswithTags (Variables|Default|GetSlayer) "(GameplayTags=((TagName=\"Ability.Inventory.CurrentWeapon.Change\")))")))

(event Input|ActionEvents|InputActionCurrentWeaponRemove
  (params (Key :type Key%20Structure :default "None"))
  (:Pressed
    (Class|BaseCharacter|ActivateAbilitieswithTags (Variables|Default|GetSlayer) "(GameplayTags=((TagName=\"Ability.Inventory.CurrentWeapon.Remove\")))")))

(fn ConstructionScript)