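; BP_Slayer is the Slayer character Blueprint, which tracks the current weapon as an index into a Weapons array.
; BeginPlay resets the index to the first slot.
; SetNextCurrentWeaponIndex advances the index, wraps to zero past the end of the array, and returns it with the weapon type from GetCurrentWeaponType.
; The graphs only handle selection state, with no spawning or equipping logic.
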(event EventBeginPlay
  (Variables|Weapon|SetCurrent%20Weapon%20Index 0))

(fn ConstructionScript)

(fn SetNextCurrentWeaponIndex
  (bind _output (Weapon|GetCurrentWeaponType))
  (bind _result (Math|Integer|IncrementInt (Variables|Weapon|GetCurrent%20Weapon%20Index))
    (:%20%20
      (if (>= _result (Utilities|Array|Length (Variables|Default|GetWeapons)))
        (bind _output_get (Variables|Weapon|SetCurrent%20Weapon%20Index 0))
        (return _output_get _output)
        (else
          (bind _output_get_2 (Variables|Weapon|SetCurrent%20Weapon%20Index _result))
          (return _output_get_2 _output))))))

(fn GetCurrentWeaponType
  (return (Utilities|Array|Get(acopy) (Variables|Default|GetWeapons) (Variables|Weapon|GetCurrent%20Weapon%20Index))))