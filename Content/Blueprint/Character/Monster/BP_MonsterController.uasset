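; AI controller for monster characters that drives their behavior and hunts slayers.
; On possessing a BP_Monster, it runs that monster's own behavior tree.
; AI perception updates set a sensed BP_Slayer as the blackboard Target and clear it when the sense is lost.
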(event OnTargetPerceptionUpdated(AIPerception)
  (params (Actor :type Actor%20Object%20Reference) (Stimulus :type AI%20Stimulus%20Structure))
  (bind _asbp_slayer (Utilities|Casting|CastToBP_Slayer Actor))
  (if (.bsuccessfullysensed Stimulus)
    (AI|Components|Blackboard|SetValueasObject (Variables|Default|GetBlackboard) (Utilities|Name|MakeLiteralName "Target") _asbp_slayer)
    (else
      (AI|Components|Blackboard|ClearValue (Variables|Default|GetBlackboard) (Utilities|Name|MakeLiteralName "Target")))))

(event EventPossess
  (params (PossessedPawn :type Pawn%20Object%20Reference))
  (bind _asbp_monster (Utilities|Casting|CastToBP_Monster PossessedPawn))
  (AI|RunBehaviorTree (Variables|/Game/Blueprint/Character/Monster/BP_Monster.BP_Monster_C|GetBehaviorTree _asbp_monster)))

(fn ConstructionScript)