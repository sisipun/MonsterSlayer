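; BP_SlayerController is the player controller for the Slayer character, handling its UI and combat input.
; On BeginPlay it creates the WB_Slayer widget, gives it a reference to itself and adds it to the viewport.
; On possess it caches the pawn as a Slayer, then routes Attack input to Slayer.Attack.
; Roll input plays the roll montage directly when CanUseAbility allows it.
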(event EventBeginPlay
  (bind _returnvalue (Game|ConstructObjectfromClass "/Game/Blueprint/Characters/Slayer/WB_Slayer.WB_Slayer_C" self))
  (bind _output_get (Variables|Default|SetSlayerUI _returnvalue))
  (Variables|/Game/Blueprint/Characters/Slayer/WB_Slayer.WB_Slayer_C|SetSlayerController _output_get self)
  (UserInterface|Viewport|AddtoViewport _output_get 0))

(event EventPossess
  (params (PossessedPawn :type Pawn%20Object%20Reference))
  (bind _asslayer (Utilities|Casting|CastToSlayer PossessedPawn))
  (Variables|Default|SetSlayer _asslayer))

(event Input|ActionEvents|InputActionRoll
  (params (Key :type Key%20Structure))
  (:Pressed
    (if (Class|BaseCharacter|CanUseAbility (Variables|Default|GetSlayer))
      (Animation|PlayAnimMontage (Variables|Default|GetSlayer) "/Game/Character/Slayer/Animations/AM_Slayer_Roll.AM_Slayer_Roll" 1.0 "None"))))

(event Input|ActionEvents|InputActionAttack
  (params (Key :type Key%20Structure))
  (:Pressed
    (Class|BaseCharacter|Attack (Variables|Default|GetSlayer))))

(fn ConstructionScript)