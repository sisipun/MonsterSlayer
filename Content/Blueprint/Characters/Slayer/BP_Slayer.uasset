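; BP_Slayer is the Slayer character Blueprint, which tracks the currently selected weapon.
; It resets the weapon index to the first slot on BeginPlay.
; Next and previous functions step the index through the Weapons array, wrapping at both ends, and return the new index.
; A getter returns the weapon type stored at the current index.
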(event EventBeginPlay
  (Variables|Weapon|SetCurrent%20Weapon%20Index 0))

(fn ConstructionScript)

(fn SetNextCurrentWeaponIndex
  (bind _result (Math|Integer|IncrementInt (Variables|Weapon|GetCurrent%20Weapon%20Index))
    (:%20%20
      (if (>= _result (Utilities|Array|Length (Variables|Default|GetWeapons)))
        (bind _output_get (Variables|Weapon|SetCurrent%20Weapon%20Index 0))
        (return _output_get)
        (else
          (bind _output_get_2 (Variables|Weapon|SetCurrent%20Weapon%20Index _result))
          (return _output_get_2))))))

(fn SetPreviousCurrentWeaponIndex
  (bind _result (Math|Integer|DecrementInt (Variables|Weapon|GetCurrent%20Weapon%20Index))
    (:%20%20
      (if (< _result 0)
        (bind _output_get (Variables|Weapon|SetCurrent%20Weapon%20Index (- (Utilities|Array|Length (Variables|Default|GetWeapons)) 1)))
        (return _output_get)
        (else
          (bind _output_get_2 (Variables|Weapon|SetCurrent%20Weapon%20Index _result))
          (return _output_get_2))))))

(fn GetCurrentWeaponType
  (return (Utilities|Array|Get(acopy) (Variables|Default|GetWeapons) (Variables|Weapon|GetCurrent%20Weapon%20Index))))