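; Player controller for the Slayer character that creates its HUD and handles its Attack and Roll input.
; On BeginPlay it spawns the Slayer widget, hands it a reference to itself and adds it to the viewport.
; On possession it caches the pawn as a Slayer, which receives Attack directly and plays the roll montage only when it can use an ability.
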(event EventBeginPlay
  (bind _returnvalue (Game|ConstructObjectfromClass "/Game/Blueprint/Characters/Slayer/Slayer_WB.Slayer_WB_C" self))
  (bind _output_get (Variables|Default|SetSlayerUI _returnvalue))
  (Variables|/Game/Blueprint/Characters/Slayer/Slayer_WB.Slayer_WB_C|SetSlayerController _output_get self)
  (UserInterface|Viewport|AddtoViewport _output_get 0))

(event EventPossess
  (params (PossessedPawn :type Pawn%20Object%20Reference))
  (bind _asslayer (Utilities|Casting|CastToSlayer PossessedPawn))
  (Variables|Default|SetSlayer _asslayer))

(event Input|ActionEvents|InputActionRoll
  (params (Key :type Key%20Structure :default "None"))
  (:Pressed
    (if (Class|BaseCharacter|CanUseAbility (Variables|Default|GetSlayer))
      (Animation|PlayAnimMontage (Variables|Default|GetSlayer) "/Game/Characters/Slayer/Animations/Slayer_Roll_AM.Slayer_Roll_AM" 1.0 "None"))))

(event Input|ActionEvents|InputActionAttack
  (params (Key :type Key%20Structure :default "None"))
  (:Pressed
    (Class|BaseCharacter|Attack (Variables|Default|GetSlayer))))

(fn ConstructionScript)